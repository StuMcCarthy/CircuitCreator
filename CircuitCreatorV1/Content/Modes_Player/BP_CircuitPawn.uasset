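; BP_CircuitPawn is a player pawn that provides clamped look control and an on-screen HMD widget.
; On BeginPlay it creates the HMD widget for player controller 0, stores it and adds it to the viewport.
; Look axis inputs are scaled by separate multipliers and added to relative rotation, splitting yaw onto the Head component and pitch onto the Neck, each clamped to a limited range.
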(event EventBeginPlay
  (bind _returnvalue (UserInterface|CreateWidget "/Game/UI/HMD.HMD_C" (Game|GetPlayerController 0)))
  (bind _output_get (Variables|Default|SetHMD%20UI _returnvalue))
  (UserInterface|Viewport|AddtoViewport _output_get 0))

(event Input|AxisEvents|InputAxisLookLeft
  (params (AxisValue :type Float%20%28single-precision%29))
  (Transformation|SetRelativeRotation (Variables|Default|GetHead) (Math|Rotator|MakeRotator 0.0 0.0 (Math|Float|Clamp(Float) (+ (* AxisValue (Variables|Default|GetLR%20Look%20Multiplier)) (.yaw (Variables|/Script/Engine.SceneComponent|GetRelativeRotation (Variables|Default|GetHead)))) -7e+01 7e+01)) false false))

(event Input|AxisEvents|InputAxisLookUp
  (params (AxisValue :type Float%20%28single-precision%29))
  (Transformation|SetRelativeRotation (Variables|Default|GetNeck) (Math|Rotator|MakeRotator 0.0 (Math|Float|Clamp(Float) (+ (* AxisValue (Variables|Default|GetUP%20DWN%20Multiplier)) (.pitch (Variables|/Script/Engine.SceneComponent|GetRelativeRotation (Variables|Default|GetNeck)))) -8e+01 8e+01) 0.0) false false))

(fn ConstructionScript)