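; Light bulb Blueprint whose point light brightness responds to the voltage of a referenced electricity Blueprint.
; Every Tick it computes power from that voltage and the bulb resistance as voltage squared over resistance, storing it in PowerCurrent.
; GetLPWValue multiplies that power by the nominal efficiency, and the result sets the point light's intensity.
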(event EventBeginPlay)

(event Collision|EventActorBeginOverlap
  (params (OtherActor :type Actor%20Object%20Reference)))

(event EventTick
  (params (DeltaSeconds :type Float%20%28single-precision%29))
  (Variables|Default|SetPower%20Current (/ (Math|Float|Square (Variables|/Game/Electrical/Electricity_BP.Electricity_BP_C|GetVoltage (Variables|Default|GetElectricity_BP))) (Variables|Default|GetBulb%20Resistance)))
  (Rendering|Components|Light|SetIntensity (Variables|Default|GetPointLight) (CallFunction|GetLPWValue)))

(fn ConstructionScript)

(fn GetLPWValue
  (return (* (Variables|Default|GetPower%20Current) (Variables|Default|GetNominal%20Efficency))))